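; BP_CollectableCoin_G is a collectable coin pickup that awards points to the player on touch.
; When its Sphere component overlaps a valid actor tagged Player, it casts the game mode to BP_ThirdPersonGameMode and adds a fixed amount to its Points.
; It then plays a 2D coin sound and destroys itself.
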(event `self.Sphere.OnComponentBeginOverlap`
  (params (OverlappedComponent :type "PrimitiveComponent Object Reference") (OtherActor :type "Actor Object Reference") (OtherComp :type "PrimitiveComponent Object Reference") (OtherBodyIndex :type Integer) (bFromSweep :type Boolean) (SweepResult :type "HitResult Structure (by ref)"))
  (if (`KismetSystemLibrary.IsValid` OtherActor)
    (if (`self.ActorHasTag` OtherActor "Player")
      (bind _asbp_third_person_game_mode (cast `/Game/ThirdPerson/Blueprints/BP_ThirdPersonGameMode` (`GameplayStatics.GetGameMode`)))
      (set `/Game/ThirdPerson/Blueprints/BP_ThirdPersonGameMode.Points` (+ (`/Game/ThirdPerson/Blueprints/BP_ThirdPersonGameMode.Points` _asbp_third_person_game_mode) 10) _asbp_third_person_game_mode)
      (`GameplayStatics.PlaySound2D` "/Game/Game/Audio/Coin.Coin" 1.0 1.0 0.0 null null)
      (`self.K2_DestroyActor`))))

(fn `UserConstructionScript`)